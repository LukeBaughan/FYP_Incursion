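; Game mode for a tower defence level that runs setup, starts the wave countdown and handles lives, win/lose, pause and level changes.
; PreGame spawns stats, store, player, UI and wave manager actors, then wires them through initialise calls and event dispatchers.
; Wave manager events feed points, wave UI and win logic; losing all lives pauses and shows the lose screen.
; Grid nodes overlapping no-build zones are marked occupied at startup.
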(event `self.ReceiveBeginPlay`
  ;[1 1 1] Begin Play
  (`self.PreGame`)
  (`self.InGame`))

(event `PreGame`
  ;[1 1 1] Pre Game
  (`self.SetUpStatsManager`)
  (`self.GetGameInstance`)
  (`self.SetUpNonBuildZone`)
  (`self.SpawnStoreManager`)
  (`self.SpawnPlayerManager`)
  (`self.SetUpPlayerManager`)
  (`self.SetUpUI_Manager`)
  (`self.SetUpWaveManager`)
  (`/Game/Luke/Player/A_PlayerManager.SetUpEventDispatchers` (`self.PlayerManager`) self (`self.StoreManager`) (`self.WaveManager`) (`self.StatsManager`))
  (`self.SetUpStoreManager`))

(event `InGame`
  ;[1 1 1] In Game
  (`/Game/Luke/Wave/A_WaveManager.BeginWaveCountdown` (`self.WaveManager`)))

(fn `GetGameInstance`
  (bind _asgi_incursion (cast `/Game/Luke/GI_Incursion` (`GameplayStatics.GetGameInstance`)))
  (set `self.GameIntance` _asgi_incursion))

(fn `LoseLives`
  (params (Amount :type Integer))
  (bind _output_get (set `self.Lives` (- (`self.Lives`) Amount)))
  (if (<= _output_get 0)
    (`/Game/Luke/PlayerStats/A_StatsManager.IncrementGamesPlayed` (`self.StatsManager`))
    ;[1 1 1] Displays the lose screen when the player is out of lives
    (`GameplayStatics.SetGamePaused` true)
    (`/Game/Luke/UI/A_UI_Manager.ShowLoseScreen` (`self.UI_Manager`))
    (else
      (`/Game/Luke/UI/HUD/W_HUD_Lives.SetLives` (`/Game/Luke/UI/HUD/W_HUD.W_HUD_Lives` (`/Game/Luke/UI/A_UI_Manager.HUD` (`self.UI_Manager`))) _output_get))))

(fn `OnGameWon`
  ;[1 1 1] Only counts as a win if the player has lives left
  (if (> (`self.Lives`) 0)
    (`/Game/Luke/PlayerStats/A_StatsManager.IncrementGamesWon` (`self.StatsManager`))
    ;[1 1 1] Displays the win screen when the player survives all waves
    (`GameplayStatics.SetGamePaused` true)
    (`/Game/Luke/UI/A_UI_Manager.ShowWinScreen` (`self.UI_Manager`))))

(fn `OpenMainMenu`
  (`GameplayStatics.OpenLevel` "Level_MainMenu"))

(fn `RestartLevel`
  (`GameplayStatics.OpenLevel` "Level_2"))

(fn `SetUpNonBuildZone`
  (locals (CurrentNode :type "/Game/Luke/Grid/A_GridNode Object Reference"))
  ;[1 1 1] Sets eevry node in a non-build zone to occupied
  (bind _outactors (`GameplayStatics.GetAllActorsOfClass` "/Game/Luke/Grid/A_GridNode.A_GridNode_C"))
  (for _array_element _outactors
    (bind _output_get (set `local.CurrentNode` _array_element))
    (if (`KismetArrayLibrary.Array_IsNotEmpty` (`self.GetOverlappingActors` _output_get "/Game/Luke/Grid/A_NoBuildZone.A_NoBuildZone_C"))
      (`/Game/Luke/Grid/I_GridNode.SetOccupied` (`local.CurrentNode`) true null))))

(fn `SetUpPlayerManager`
  (`/Game/Luke/Player/A_PlayerManager.Initialise` (`self.PlayerManager`) (`/Game/Luke/GI_Incursion.GetSpawnWeapon` (`self.GameIntance`))))

(fn `SetUpStatsManager`
  (bind _returnvalue (`|SpawnActorFromClass` "/Game/Luke/PlayerStats/A_StatsManager.A_StatsManager_C" (`KismetMathLibrary.MakeTransform` (0.0 0.0 0.0)) "Undefined" "OverrideRootScale" null null))
  (bind _output_get (set `self.StatsManager` _returnvalue))
  (`/Game/Luke/PlayerStats/A_StatsManager.Initialise` _output_get))

(fn `SetUpStoreManager`
  (bind _storemanager (`self.StoreManager`))
  (`/Game/Luke/Store/A_StoreManager.Initialise` _storemanager (`/Game/Luke/Player/C_PlayerCharacter.TowerPreviewLocation` (`/Game/Luke/Player/A_PlayerManager.PlayerCharacter` (`self.PlayerManager`))) (`self.UI_Manager`))
  ;[1 1 1] Called when the player previews / places a tower
  (add `/Game/Luke/Store/A_StoreManager.OnRequestSetPlayerHoldingTower` _storemanager (`|CreateDelegate` (`/Game/Luke/Player/A_PlayerManager.PlayerCharacter` (`self.PlayerManager`)) :!event `SetHoldingTower`)))

(fn `SetUpUI_Manager`
  (bind _hud (`/Game/Luke/UI/A_UI_Manager.HUD` (`self.UI_Manager`)))
  ;[1 1 1] Cpawns and sets up the UI manager
  (bind _returnvalue (`|SpawnActorFromClass` "/Game/Luke/UI/A_UI_Manager.A_UI_Manager_C" (`KismetMathLibrary.MakeTransform` (0.0 0.0 0.0)) "Undefined" "OverrideRootScale" null null))
  (bind _output_get (set `self.UI_Manager` _returnvalue))
  (`/Game/Luke/UI/A_UI_Manager.Initialise` _output_get (`/Game/Luke/Player/A_PlayerManager.PlayerController` (`self.PlayerManager`)))
  (`/Game/Luke/UI/A_UI_Manager.SetUpEventDispatchers` _output_get (`self.StoreManager`) self)
  (set `/Game/Luke/Player/A_PlayerManager.W_UI_HUD` _hud (`self.PlayerManager`))
  (`/Game/Luke/UI/HUD/W_HUD_Lives.SetLives` (`/Game/Luke/UI/HUD/W_HUD.W_HUD_Lives` _hud) (`self.Lives`)))

(fn `SetUpWaveManager`
  (bind _wavemanager (`self.WaveManager`))
  (bind _hud (`/Game/Luke/UI/A_UI_Manager.HUD` (`self.UI_Manager`)))
  ;[1 1 1] Sets up the wave manager actor
  (bind _returnvalue (`|SpawnActorFromClass` "/Game/Luke/Wave/A_WaveManager.A_WaveManager_C" (`KismetMathLibrary.MakeTransform` (0.0 0.0 0.0)) "Undefined" "OverrideRootScale" null null))
  (bind _output_get (set `self.WaveManager` _returnvalue))
  (`/Game/Luke/Wave/A_WaveManager.Initialise` _output_get self (`/Game/Luke/UI/HUD/W_HUD.W_HUD_Timer` _hud) (`/Game/Luke/UI/HUD/W_HUD.W_SkipCountdown` _hud))
  ;[1 1 1] Called when an enemy is defeated
  (add `/Game/Luke/Wave/A_WaveManager.OnRequestPoints` _wavemanager (`|CreateDelegate` (`self.StoreManager`) :!event `AddPoints`))
  (add `/Game/Luke/Wave/A_WaveManager.OnRequestPoints` _wavemanager (`|CreateDelegate` (`self.StatsManager`) :!event `IncreaseTotalPoints`))
  (add `/Game/Luke/Wave/A_WaveManager.OnEnemyDefeated` _wavemanager (`|CreateDelegate` (`self.StatsManager`) :!event `IncrementEnemiesKilled`))
  ;[1 1 1] Shows the win screen if the player finishes all waves
  (add `/Game/Luke/Wave/A_WaveManager.OnGameWon` _wavemanager (`|CreateDelegate` :!event `OnGameWon`))
  ;[1 1 1] Updates the UI HUD wave counter
  (add `/Game/Luke/Wave/A_WaveManager.OnWaveBegin` _wavemanager (`|CreateDelegate` (`/Game/Luke/UI/HUD/W_HUD.W_HUD_Wave` (`/Game/Luke/UI/A_UI_Manager.HUD` (`self.UI_Manager`))) :!event `SetWave`))
  ;[1 1 1] Replenishes the player's health when a new wave begins
  (add `/Game/Luke/Wave/A_WaveManager.OnWaveEnded` (`self.WaveManager`) (`|CreateDelegate` (`self.PlayerManager`) :!event `ReplenishPlayerHealth`))
  ;[1 1 1] Gives the player points when a new wave begins
  (add `/Game/Luke/Wave/A_WaveManager.OnWaveEnded` (`self.WaveManager`) (`|CreateDelegate` (`self.StoreManager`) :!event `AddNewWavePoints`)))

(fn `SpawnPlayerManager`
  (bind _returnvalue (`|SpawnActorFromClass` "/Game/Luke/Player/A_PlayerManager.A_PlayerManager_C" (`KismetMathLibrary.MakeTransform` (0.0 0.0 0.0)) "Undefined" "OverrideRootScale" null null))
  (set `self.PlayerManager` _returnvalue))

(fn `SpawnStoreManager`
  (bind _returnvalue (`|SpawnActorFromClass` "/Game/Luke/Store/A_StoreManager.A_StoreManager_C" (`KismetMathLibrary.MakeTransform` (0.0 0.0 0.0)) "Undefined" "OverrideRootScale" null null))
  (set `self.StoreManager` _returnvalue))

(fn `TogglePauseGame`
  (params (Pause :type Boolean))
  (bind _ui_manager (`self.UI_Manager`))
  (`GameplayStatics.SetGamePaused` Pause)
  (`/Game/Luke/UI/A_UI_Manager.ToggleMenu` _ui_manager (`/Game/Luke/UI/A_UI_Manager.UI_PauseMenu` _ui_manager)))

(fn `UserConstructionScript`)